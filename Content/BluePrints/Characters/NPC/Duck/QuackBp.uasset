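; QuackBp is a duck NPC that drops a raw duck item when killed.
; AnyDamage subtracts damage from Health, and at zero or below destroys the actor, then spawns Item_DuckRaw.
; The drop uses the mesh's world transform cached at BeginPlay, so it appears where the duck started rather than where it died.
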(event EventBeginPlay
  (Variables|Default|SetWhere%20to%20Spawn (Transformation|GetWorldTransform (Variables|Character|GetMesh self))))

(event Collision|EventActorBeginOverlap
  (params (OtherActor :type Actor%20Object%20Reference)))

(event EventTick
  (params (DeltaSeconds :type Float%20%28single-precision%29)))

(event Game|Damage|EventAnyDamage
  (params (Damage :type Float%20%28single-precision%29) (DamageType :type Damage%20Type%20Object%20Reference) (InstigatedBy :type Controller%20Object%20Reference) (DamageCauser :type Actor%20Object%20Reference))
  (bind _output_get (Variables|Default|SetHealth (- (Variables|Default|GetHealth) Damage)))
  (if (<= _output_get 0.0)
    (Actor|DestroyActor self)
    (Game|SpawnActorfromClass :Class "/Game/BluePrints/Items/Food/Item_DuckRaw.Item_DuckRaw_C" :SpawnTransform (Variables|Default|GetWhere%20to%20Spawn) :CollisionHandlingOverride "Undefined" :screenmessageRef 0 :Instigator 0)))

(fn ConstructionScript)