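; Game instance that manages menus, the saved player profile and multiplayer sessions.
; SaveGameCheck opens the main menu if a save exists, otherwise player options, with widgets cached for reuse.
; Save and load functions copy player info and name through FF_SaveGame, loading only when SaveGameRef is already valid.
; Advanced session nodes host a listen server, join and find servers, while network and travel errors destroy the session and return to MainMenu.
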(event Custom|QuitGame
  (bind _returnvalue (Game|GetPlayerController 0))
  ;[1 1 1] Quit The Game
  (if (Pawn|IsLocalPlayerController _returnvalue)
    (Game|QuitGame _returnvalue "Quit" false)))

(event Custom|ShowPlayerOptions
  (params (PlayerController :type Player%20Controller%20Object%20Reference))
  (bind _returnvalue (Game|GetPlayerController 0))
  ;[1 1 1] Show PlayerOptions
  (Utilities|IsValid (Variables|Widgets|GetPlayerSettings_W)
    (:Is%20Valid
      _)
    (:Is%20Not%20Valid
      (bind _returnvalue_2 (UserInterface|CreateWidget "/Game/Ui/MainMenu/PlayerSettings.PlayerSettings_C" PlayerController))
      (bind _output_get (Variables|Widgets|SetPlayerSettings_W _returnvalue_2))))
  (UserInterface|Viewport|AddtoViewport (Variables|Widgets|GetPlayerSettings_W) 0)
  (Variables|/Script/Engine.PlayerController|SetbShowMouseCursor _returnvalue true)
  (Input|SetInputModeUIOnly _returnvalue _output_get "DoNotLock"))

(event Custom|ShowMainMenu
  (bind _returnvalue (Game|GetPlayerController 0))
  ;[1 1 1] ShowMainMenu
  (Utilities|IsValid (Variables|Widgets|GetMainMenu_W)
    (:Is%20Valid
      _)
    (:Is%20Not%20Valid
      (bind _returnvalue_2 (UserInterface|CreateWidget "/Game/Ui/MainMenu/MainMenu.MainMenu_C" (Variables|PlayerInfo|GetOwnerRef)))
      (bind _output_get (Variables|Widgets|SetMainMenu_W _returnvalue_2))))
  (UserInterface|Viewport|AddtoViewport (Variables|Widgets|GetMainMenu_W) 0)
  (Variables|/Script/Engine.PlayerController|SetbShowMouseCursor _returnvalue true)
  (Input|SetInputModeUIOnly _returnvalue _output_get "DoNotLock"))

(event Custom|FindServers
  (params (PlayerController :type Player%20Controller%20Object%20Reference) (MaxResults :type Integer))
  ;[1 1 1] Find Servers
  (bind _results (|FindSessionsAdvanced PlayerController MaxResults false "AllServers" 0 false false false)
    (:OnSuccess
      _)
    (:OnFailure
      _))
  (Default|CallServersFound _results))

(event Custom|QuitToMenu
  (params (PlayerController :type Player%20Controller%20Object%20Reference))
  ;[1 1 1] Quit back to Mainmenu/Or if session fails - back to main menu
  (if (Pawn|IsLocalPlayerController PlayerController)
    (|DestroySession PlayerController
      (:OnSuccess
        _)
      (:OnFailure
        _))
    (Game|OpenLevel(byName) "MainMenu")))

(event Custom|ShowHostMenu
  ;[1 1 1] ShowHostMenu
  (Utilities|IsValid (Variables|Widgets|GetHostMenu_w)
    (:Is%20Valid
      _)
    (:Is%20Not%20Valid
      (bind _returnvalue (UserInterface|CreateWidget "/Game/Ui/MainMenu/HostGame.HostGame_C" (Game|GetPlayerController 0)))
      (Variables|Widgets|SetHostMenu_w _returnvalue)))
  (UserInterface|Viewport|AddtoViewport (Variables|Widgets|GetHostMenu_w) 0))

(event Custom|ShowOnline
  ;[1 1 1] showOnlin
  (Utilities|IsValid (Variables|Widgets|GetOnline_W)
    (:Is%20Valid
      _)
    (:Is%20Not%20Valid
      (bind _returnvalue (UserInterface|CreateWidget "/Game/Ui/MainMenu/OnlineMenu.OnlineMenu_C" (Game|GetPlayerController 0)))
      (Variables|Widgets|SetOnline_W _returnvalue)))
  (UserInterface|Viewport|AddtoViewport (Variables|Widgets|GetOnline_W) 0))

(event Custom|HostServer
  (params (PlayerController :type Player%20Controller%20Object%20Reference) (ServerSettings :type Server%20Settings%20Structure))
  (bind (_mapname _publicconnections _serversettings) (Utilities|Struct|BreakServerSettings ServerSettings))
  ;[1 1 1] Host a session/server
  (Variables|Default|SetMyName (Variables|Default|GetMyName))
  (bind _output_get (Variables|PlayerInfo|SetOwnerRef PlayerController))
  (Input|SetInputModeGameOnly _output_get)
  (|AdvancedSession _serversettings _output_get _publicconnections 0 false true false true true false false false true
    (:OnSuccess
      (Variables|Default|SetServerSettings ServerSettings)
      (Game|OpenLevel(byName) "TestLevel" true "listen"))))

(event Custom|UpdateSaveGame
  ;[1 1 1] calls to savegame
  (CallFunction|SaveGame))

(event Custom|SaveGameCheck
  (bind _ownerref (Variables|PlayerInfo|GetOwnerRef))
  (bind _returnvalue (Class|GameplayStatics|GetPlayerControllerID _ownerref))
  (bind _returnvalue_2 (Game|GetPlayerController _returnvalue))
  ;[1 1 1] SaveGameCheck
  (bind _returnvalue_3 (SaveGame|DoesSaveGameExist (Variables|PlayerInfo|GetFF_SaveGame) _returnvalue))
  (if _returnvalue_3
    (CallFunction|ShowMainMenu)
    (Variables|Default|SetCreatedSaveFile? true)
    (else
      (CallFunction|ShowPlayerOptions _ownerref)
      (Variables|/Script/Engine.PlayerController|SetbShowMouseCursor _returnvalue_2 true)
      (Variables|Default|SetCreatedSaveFile? false)
      (Input|SetInputModeUIOnly _returnvalue_2 (Variables|Widgets|GetPlayerSettings_W) "LockOnCapture"))))

(event Custom|saveByServer
  ;[1 1 1] calls to savegame
  (CallFunction|SaveGame))

(event Custom|UpdateServerWithPlayerinfo
  ;[1 1 1] calls to savegame
)

(event Custom|JoinServer
  (params (PlayerController :type Player%20Controller%20Object%20Reference) (SearchResult :type Blueprint%20Session%20Result%20Structure%20%28by%20ref%29))
  ;[1 1 1] Join a Server
  (bind _output_get (Variables|PlayerInfo|SetOwnerRef PlayerController))
  (Input|SetInputModeGameOnly _output_get)
  (|JoinSession _output_get SearchResult))

(event EventHandleNetworkError
  (params (FailureType :type ENetworkFailure%20Enum :default "NetDriverAlreadyExists") (bIsServer :type Boolean))
  (bind _ownerref (Variables|PlayerInfo|GetOwnerRef))
  ;[1 1 1] Network Error
  (Development|PrintString (Utilities|String|Append (Utilities|String|EnumtoString FailureType) " 
" (Utilities|GetDisplayName _ownerref)))
  (CallFunction|QuittoMenu _ownerref))

(event EventInit
  (bind _returnvalue (Game|GetPlayerController 0))
  ;[1 1 1] Init Game
  (Utilities|IsValid _returnvalue
    (:Is%20Valid
      (Variables|PlayerInfo|SetOwnerRef _returnvalue))))

(event EventHandleTravelError
  (params (FailureType :type ETravelFailure%20Enum :default "NoLevel"))
  (bind _ownerref (Variables|PlayerInfo|GetOwnerRef))
  ;[1 1 1] TravelError
  (Development|PrintString (Utilities|String|Append (Utilities|String|EnumtoString FailureType) " 
" (Utilities|GetDisplayName _ownerref)))
  (CallFunction|QuittoMenu _ownerref))

(fn SaveExistThenLoad
  (bind _returnvalue (SaveGame|DoesSaveGameExist (Variables|PlayerInfo|GetFF_SaveGame)))
  (if _returnvalue
    (Utilities|IsValid (Variables|Default|GetSaveGameRef)
      (:Is%20Valid
        (bind _returnvalue_2 (SaveGame|LoadGamefromSlot (Variables|PlayerInfo|GetFF_SaveGame) (Class|GameplayStatics|GetPlayerControllerID (Variables|PlayerInfo|GetOwnerRef))))
        (bind _asff_save_game (Utilities|Casting|CastToFF_SaveGame _returnvalue_2))
        (bind _output_get (Variables|PlayerInfo|SetPlayers_PlayerInfo (Variables|/Game/BluePrints/All/FF_SaveGame.FF_SaveGame_C|GetSaved_PlayerInfo _asff_save_game)))
        (Variables|Default|SetMyName (.PlayerName (Utilities|Struct|BreakPlayerInfo _output_get)))))))

(fn SaveGame
  (bind _players_playerinfo (Variables|PlayerInfo|GetPlayers_PlayerInfo))
  (Utilities|IsValid (Variables|Default|GetSaveGameRef)
    (:Is%20Valid
      _)
    (:Is%20Not%20Valid
      (bind _returnvalue (SaveGame|CreateSaveGameObject "/Game/BluePrints/All/FF_SaveGame.FF_SaveGame_C"))
      (Variables|Default|SetSaveGameRef _returnvalue)))
  (Variables|/Game/BluePrints/All/FF_SaveGame.FF_SaveGame_C|SetSaved_PlayerInfo (Variables|Default|GetSaveGameRef) _players_playerinfo)
  (bind _returnvalue_2 (SaveGame|SaveGametoSlot (Variables|Default|GetSaveGameRef) (Variables|PlayerInfo|GetFF_SaveGame)))
  (Variables|Default|SetCreatedSaveFile? _returnvalue_2)
  (Variables|Default|SetMyName (.PlayerName (Utilities|Struct|BreakPlayerInfo _players_playerinfo))))

(fn LoadGame
  (bind _savegameref (Variables|Default|GetSaveGameRef))
  (Utilities|IsValid _savegameref
    (:Is%20Valid
      (bind _returnvalue (SaveGame|LoadGamefromSlot (Variables|PlayerInfo|GetFF_SaveGame) (Class|GameplayStatics|GetPlayerControllerID (Variables|PlayerInfo|GetOwnerRef))))
      (bind _asff_save_game (Utilities|Casting|CastToFF_SaveGame _returnvalue))
      (Variables|ForSakenGameinstnce_C|SetPlayers_PlayerInfo self (Variables|/Game/BluePrints/All/FF_SaveGame.FF_SaveGame_C|GetSaved_PlayerInfo _asff_save_game))
      (Variables|Default|SetMyName (.PlayerName (Utilities|Struct|BreakPlayerInfo (Variables|/Game/BluePrints/All/FF_SaveGame.FF_SaveGame_C|GetSaved_PlayerInfo _savegameref)))))))