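; Crafting component that toggles a crafting table window and checks whether placed items satisfy a recipe.
; ToggleCraftingTable creates or removes the HUD canvas widget, switches input mode and cursor, and toggles the player's backpack inventory.
; CheckForItemsAvailable searches the crafting slots for the current recipe's three item classes, resetting the recipe index on a match.
; Stepping through other recipes is unwired, and GivePlayerNewItem is an empty stub.
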(event EventBeginPlay)

(event EventTick
  (params (DeltaSeconds :type Float%20%28single-precision%29)))

(fn ToggleCraftingTable
  (bind _returnvalue (Game|GetPlayerController 0))
  (bind _returnvalue_2 (Game|GetPlayerController 0))
  (Variables|Default|Getcrafting%20window
    (:then
      (Widget|RemovefromParent (Variables|Default|Getcrafting%20window))
      (Variables|Default|Setcrafting%20window 0)
      (Input|SetInputModeGameOnly _returnvalue)
      (Variables|/Script/Engine.PlayerController|SetbShowMouseCursor _returnvalue false)
      (bind _asbase_player (Utilities|Casting|CastToBase_Player (Game|GetPlayerCharacter 0)))
      (Default|ToggleInventory (Variables|/Game/BluePrints/Characters/Base_Player.Base_Player_C|GetBackPackComponent _asbase_player))
      (Variables|/Game/BluePrints/InventorySystem/InventoryComponent.InventoryComponent_C|SetInventoryWindow (Variables|/Game/BluePrints/Characters/Base_Player.Base_Player_C|GetBackPackComponent _asbase_player) 0))
    (:else
      (bind _returnvalue_3 (UserInterface|CreateWidget "/Game/BluePrints/InventorySystem/InventoryUI/CraftingWindow.CraftingWindow_C" 0 self))
      (bind _output_get (Variables|Default|Setcrafting%20window _returnvalue_3))
      (bind _asff_player_controller (Utilities|Casting|CastToFF_PlayerController (Game|GetPlayerController 0)))
      (bind _returnvalue_4 (Class|CanvasPanel|AddChildtoCanvas (Variables|/Game/Ui/Ingame/InGameHud.InGameHud_C|GetHudCanvas (Variables|/Game/BluePrints/Game/FF_PlayerController.FF_PlayerController_C|GetIngameHud _asff_player_controller)) _output_get))
      (Class|CanvasPanelSlot|SetAutoSize _returnvalue_4 false)
      (Input|SetInputModeUIOnly _returnvalue_2 0 "LockAlways")
      (Variables|/Script/Engine.PlayerController|SetbShowMouseCursor _returnvalue_2 true)
      (bind _asbase_player_2 (Utilities|Casting|CastToBase_Player (Game|GetPlayerCharacter 0)))
      (Default|ToggleInventory (Variables|/Game/BluePrints/Characters/Base_Player.Base_Player_C|GetBackPackComponent _asbase_player_2)))))

(fn CheckforItemsAvailable
  (bind _craftingarray (Variables|Default|GetCraftingArray))
  (bind _craftingarray_2 (Variables|Default|GetCraftingArray))
  (bind _craftingarray_3 (Variables|Default|GetCraftingArray))
  ;[1 1 1] Check all crafting slots for given reciept slot if matches will return true
  (bind _array_index (Utilities|Array|ForEachLoopwithBreak _craftingarray_2 :!label _label)
    (:LoopBody
      (if (== (.Item1 (Utilities|Struct|BreakRecieptStructure (Utilities|Array|Get(acopy) (Variables|Default|GetRecieptsArray) (Variables|Default|GetRecieptIndex)))) (.class (.ItemStructure (Utilities|Struct|BreakSlotStructure (Utilities|Array|Get(acopy) _craftingarray_2 _array_index)))))
        (LocalVariables|SetHasItem1 true)
        (goto _label Break)))
    (:Completed
      (bind _array_index_2 (Utilities|Array|ForEachLoopwithBreak _craftingarray_3 :!label _label_2)
        (:LoopBody
          (if (== (.Item2 (Utilities|Struct|BreakRecieptStructure (Utilities|Array|Get(acopy) (Variables|Default|GetRecieptsArray) (Variables|Default|GetRecieptIndex)))) (.class (.ItemStructure (Utilities|Struct|BreakSlotStructure (Utilities|Array|Get(acopy) _craftingarray_3 _array_index_2)))))
            (LocalVariables|SetHasItem2 true)
            (goto _label_2 Break)))
        (:Completed
          (bind _array_index_3 (Utilities|Array|ForEachLoopwithBreak _craftingarray :!label _label_3)
            (:LoopBody
              (if (== (.Item3 (Utilities|Struct|BreakRecieptStructure (Utilities|Array|Get(acopy) (Variables|Default|GetRecieptsArray) (Variables|Default|GetRecieptIndex)))) (.class (.ItemStructure (Utilities|Struct|BreakSlotStructure (Utilities|Array|Get(acopy) _craftingarray _array_index_3)))))
                (LocalVariables|SetHasItem3 true)
                (goto _label_3 Break)))
            (:Completed
              (if (Math|Boolean|ANDBoolean (LocalVariables|GetHasItem1) (LocalVariables|GetHasItem2) (LocalVariables|GetHasItem3))
                (Variables|Default|SetRecieptIndex 0)
                (return true)
                (else
                  (return false))))))))))

(fn GivePlayerNewItem)