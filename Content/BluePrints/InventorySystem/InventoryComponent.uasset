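; Inventory actor component that stores slot-based items and toggles their UI for the local player.
; Adding an item fills partial stacks first, recursing on overflow, then takes the first empty slot.
; PrepareInventory sizes the array, blanks empty slots and refreshes items from class defaults, while InventoryQuery totals a class's quantity against an amount.
; The "BackPack" inventory opens alongside the character sheet; others open their own window, switching input mode and cursor.
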(event EventBeginPlay
  (CallFunction|PrepareInventory))

(fn ToggleInventory
  (bind _returnvalue (Game|GetPlayerController 0))
  (bind _returnvalue_2 (Game|GetPlayerController 0))
  (bind _returnvalue_3 (Game|GetPlayerController 0))
  (bind _returnvalue_4 (Game|GetPlayerController 0))
  (bind _self self)
  (bind _self_2 self)
  (bind _asbase_player (Utilities|Casting|CastToBase_Player (Game|GetPlayerCharacter 0)))
  (if (Pawn|IsLocallyControlled _asbase_player)
    ;[1 1 1] Check if its player backpack
    (if (Utilities|Enum|Equal(Enum) (Variables|Default|GetInventoryName self) (Utilities|Text|MakeLiteralText "BackPack"))
      (bind _asbase_player_2 (Utilities|Casting|CastToBase_Player (Game|GetPlayerCharacter 0)))
      (if (Variables|/Game/BluePrints/Characters/Base_Player.Base_Player_C|GetHasBackPack? _asbase_player_2)
        (Variables|Default|Getbackpackwindow
          (:then
            (Widget|RemovefromParent (Variables|Default|Getbackpackwindow))
            (Variables|Default|Setbackpackwindow 0)
            (Widget|RemovefromParent (Variables|Default|GetEquipmentWindow) :!label _label)
            (Variables|Default|SetEquipmentWindow 0)
            (Input|SetInputModeGameOnly _returnvalue)
            (Variables|/Script/Engine.PlayerController|SetbShowMouseCursor _returnvalue false))
          (:else
            (CallFunction|PrepareInventory)
            (bind _returnvalue_5 (UserInterface|CreateWidget "/Game/BluePrints/InventorySystem/InventoryUI/Backpack/BackPackWindow.BackPackWindow_C" 0 _self (Variables|Default|GetInventoryName _self)))
            (bind _output_get (Variables|Default|Setbackpackwindow _returnvalue_5))
            (Variables|Default|GetEquipmentWindow :!label _label_2
              (:then
                (goto _label))
              (:else
                (bind _returnvalue_6 (UserInterface|CreateWidget "/Game/BluePrints/CharacterEquipment/CharacterSheet.CharacterSheet_C"))
                (bind _output_get_2 (Variables|Default|SetEquipmentWindow _returnvalue_6))
                (bind _asff_player_controller (Utilities|Casting|CastToFF_PlayerController (Game|GetPlayerController 0)))
                (if (Pawn|IsLocalPlayerController _asff_player_controller)
                  (Class|CanvasPanel|AddChildtoCanvas (Variables|/Game/Ui/Ingame/InGameHud.InGameHud_C|GetHudCanvas (Variables|/Game/BluePrints/Game/FF_PlayerController.FF_PlayerController_C|GetIngameHud _asff_player_controller)) _output_get)
                  (Class|CanvasPanel|AddChildtoCanvas (Variables|/Game/Ui/Ingame/InGameHud.InGameHud_C|GetHudCanvas (Variables|/Game/BluePrints/Game/FF_PlayerController.FF_PlayerController_C|GetIngameHud _asff_player_controller)) _output_get_2)
                  (Input|SetInputModeGameandUI _returnvalue_2 0 "DoNotLock" true)
                  (Variables|/Script/Engine.PlayerController|SetbShowMouseCursor _returnvalue_2 true))))))
        (else
          (goto _label_2)))
      (else
        (Variables|Default|GetInventoryWindow
          (:then
            (Widget|RemovefromParent (Variables|Default|GetInventoryWindow))
            (Variables|Default|SetInventoryWindow 0)
            (Input|SetInputModeGameOnly _returnvalue_4)
            (Variables|/Script/Engine.PlayerController|SetbShowMouseCursor _returnvalue_4 false))
          (:else
            (CallFunction|PrepareInventory)
            (bind _returnvalue_7 (UserInterface|CreateWidget "/Game/BluePrints/InventorySystem/InventoryUI/Inventory/InventoryWindow.InventoryWindow_C" 0 _self_2 (Variables|Default|GetInventoryName _self_2)))
            (bind _output_get_3 (Variables|Default|SetInventoryWindow _returnvalue_7))
            (bind _asff_player_controller_2 (Utilities|Casting|CastToFF_PlayerController (Game|GetPlayerController 0)))
            (if (Pawn|IsLocalPlayerController _asff_player_controller_2)
              (bind _returnvalue_8 (Class|CanvasPanel|AddChildtoCanvas (Variables|/Game/Ui/Ingame/InGameHud.InGameHud_C|GetHudCanvas (Variables|/Game/BluePrints/Game/FF_PlayerController.FF_PlayerController_C|GetIngameHud _asff_player_controller_2)) _output_get_3))
              (Class|CanvasPanelSlot|SetAutoSize _returnvalue_8 true)
              (Input|SetInputModeUIOnly _returnvalue_3 (Variables|Default|GetInventoryWindow) "LockAlways")
              (Variables|/Script/Engine.PlayerController|SetbShowMouseCursor _returnvalue_3 true))))))))

(fn AddtoInventory
  (params (ContentToAdd :type Slot%20Structure%20Structure))
  (if (.isstackable? (.itemstructure ContentToAdd))
    (bind _stackindex (Utilities|HasPartialStack ContentToAdd)
      (:True
        (bind _sucsess (CallFunction|AddtoStack ContentToAdd _stackindex))
        (if _sucsess
          _
          (else
            (Development|PrintString "doesnt work on partial")
            (return false))))
      (:False
        (bind _sucsess_2 (CallFunction|CreateStack ContentToAdd :!label _label))
        (if _sucsess_2
          _
          (else
            (Development|PrintString "cant seem to add")
            (return false)))))
    (else
      (goto _label)))
  (return true))

(fn PrepareInventory
  (bind _inventory (Variables|Default|GetInventory))
  (Utilities|Array|Resize (Variables|Default|GetInventory) (Variables|Default|GetNumberOfSlots))
  (for (_array_element _array_index) (Variables|Default|GetInventory)
    (if (< (.quantity _array_element) 1)
      (bind _structout (Utilities|Struct|SetmembersinSlotStructure (Utilities|Array|Get(acopy) (Variables|Default|GetInventory) _array_index) (Utilities|Struct|MakeItemStructure "" "" 0 false 4 true 1e+01 false 0.0 false 0.0 false false 0.0 "NewEnumerator0" false "NewEnumerator3" 0.0 false "NewEnumerator0" false "NewEnumerator0" false "NewEnumerator0" 0 false "NewEnumerator0" 0.0 0 0 0)))
      (Utilities|Array|SetArrayElem _inventory _array_index _structout)
      (elif (!= (.Class (Utilities|Struct|BreakItemStructure (.itemstructure _array_element))) 0)
        (Utilities|Array|SetArrayElem _inventory _array_index (Utilities|Struct|MakeSlotStructure (.ItemStructure (Utilities|GetClassDefaults (.Class (Utilities|Struct|BreakItemStructure (.itemstructure _array_element))))) (.quantity _array_element)))))))

(fn CreateStack
  (params (ContentToAdd :type Slot%20Structure%20Structure))
  (bind (_array_element _array_index) (Utilities|Array|ForEachLoopwithBreak (Variables|Default|GetInventory) :!label _label)
    (:LoopBody
      (if (<= (.quantity _array_element) 0)
        (LocalVariables|SetHasSpace? true)
        (goto _label Break)))
    (:Completed
      (if (LocalVariables|GetHasSpace?)
        (Utilities|Array|SetArrayElem (Variables|Default|GetInventory) _array_index ContentToAdd)
        (return (LocalVariables|GetHasSpace?))
        (else
          (return false))))))

(fn AddtoStack
  (params (SlotStructure :type Slot%20Structure%20Structure) (SlotIndex :type Integer))
  (bind _inventory (Variables|Default|GetInventory))
  (bind _inventory_2 (Variables|Default|GetInventory))
  (bind _maxstacksize (Utilities|Struct|BreakItemStructure (.itemstructure SlotStructure)))
  (bind _output (Utilities|Array|Get(acopy) _inventory SlotIndex))
  (bind _output_2 (Utilities|Array|Get(acopy) _inventory_2 SlotIndex))
  (bind _output_get (LocalVariables|SetCurrentQuantity (.quantity _output)))
  (if (> (+ _output_get (.Quantity (Utilities|Struct|BreakSlotStructure SlotStructure))) (.maxstacksize (.itemstructure _output)))
    (Utilities|Array|SetArrayElem (Variables|Default|GetInventory) SlotIndex (Utilities|Struct|MakeSlotStructure (.itemstructure SlotStructure) _maxstacksize))
    (CallFunction|AddtoInventory (Utilities|Struct|MakeSlotStructure (.itemstructure SlotStructure) (- (.quantity SlotStructure) (- _maxstacksize (LocalVariables|GetCurrentQuantity)))))
    (else
      (Utilities|Array|SetArrayElem _inventory_2 SlotIndex (Utilities|Struct|MakeSlotStructure (.itemstructure _output_2) (+ (.quantity SlotStructure) (.quantity _output_2))))))
  (return true))

(fn InventoryQuery
  (params (ItemClass :type Item%20Class%20Reference) (QueryAmount :type Integer))
  (bind _array_element (Utilities|Array|ForEachLoopwithBreak (Variables|Default|GetInventory))
    (:LoopBody
      (if (== (.Class (Utilities|Struct|BreakItemStructure (.itemstructure _array_element))) ItemClass)
        (LocalVariables|SetRunningTotal (+ (.quantity _array_element) (LocalVariables|GetRunningTotal)))))
    (:Completed
      (if (>= QueryAmount (LocalVariables|GetRunningTotal))
        (return true)
        (else
          (return false))))))