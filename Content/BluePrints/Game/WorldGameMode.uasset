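; World game mode for a multiplayer server that tracks joining players and spawns their characters.
; PostLogin, on authority, registers the controller, caches PlayerStarts, reads server name and player limit from the game instance, then starts the controller's initial setup.
; RespawnPlayer destroys any current pawn, then spawns and possesses a male or female character by chosen gender at a random start.
; EveryOneUpdate rebuilds the connected-player list and pushes it, with player counts, to every controller.
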(event Custom|RespawnPlayer
  (params (PlayerController :type Player%20Controller%20Object%20Reference))
  (bind _spawnpoints (Variables|ServerSettings|GetSpawnPoints))
  (bind _returnvalue (Utilities|Array|Length _spawnpoints))
  (bind _returnvalue_2 (- _returnvalue 1))
  (bind _returnvalue_3 (Math|Random|RandomIntegerinRange 0 _returnvalue_2))
  (bind _output (Utilities|Array|Get(acopy) _spawnpoints _returnvalue_3))
  (bind _returnvalue_4 (Transformation|GetActorTransform _output))
  ;[1 1 1] the actual spawn
  (bind _asff_player_controller (Utilities|Casting|CastToFF_PlayerController PlayerController))
  (Utilities|IsValid _asff_player_controller
    (:Is%20Valid
      (Utilities|IsValid (Pawn|GetControlledPawn _asff_player_controller)
        (:Is%20Valid
          (Actor|DestroyActor (Pawn|GetControlledPawn _asff_player_controller)))
        (:Is%20Not%20Valid
          _)))
    (:Is%20Not%20Valid
      _))
  (switch Utilities|FlowControl|Switch|SwitchonPlayersGender (.PlayersChosenGender (Utilities|Struct|BreakPlayerInfo (Variables|/Game/BluePrints/Game/FF_PlayerController.FF_PlayerController_C|GetPlayerSettings _asff_player_controller)))
    (:NewEnumerator1
      (bind _returnvalue_5 (Game|SpawnActorfromClass "/Game/BluePrints/Characters/Tribes/FemalePlayer.FemalePlayer_C" _returnvalue_4 "AdjustIfPossibleButAlwaysSpawn" 0 0 1e+02 75.0 1.0 false false 0 0 false 0))
      (Pawn|Possess PlayerController _returnvalue_5))
    (:NewEnumerator2
      (bind _returnvalue_6 (Game|SpawnActorfromClass "/Game/BluePrints/Characters/Tribes/MalePlayer.MalePlayer_C" _returnvalue_4 "AdjustIfPossibleButAlwaysSpawn" 0 0 1e+02 75.0 1.0 false false 0 0 false 0))
      (Pawn|Possess PlayerController _returnvalue_6))))

(event Custom|EveryOneUpdate
  (bind _allplayercontrollers (Variables|ServerSettings|GetAllPlayerControllers))
  ;[1 1 1] update all on server
  (bind _output_get (Variables|ServerSettings|SetCurrentPlayers (Utilities|Array|Length (Variables|ServerSettings|GetAllPlayerControllers))))
  (if (> _output_get 0)
    (Utilities|Array|Clear (Variables|ServerSettings|GetConnectedPlayers))
    (for _array_element _allplayercontrollers
      (bind _asff_player_controller (Utilities|Casting|CastToFF_PlayerController _array_element))
      (Utilities|Array|Add (Variables|ServerSettings|GetConnectedPlayers) (Variables|/Game/BluePrints/Game/FF_PlayerController.FF_PlayerController_C|GetPlayerSettings _asff_player_controller))
      (Default|UpdateNumberOfPlayers _asff_player_controller (Variables|ServerSettings|GetCurrentPlayers) (Variables|ServerSettings|GetServerMaxPlayers)))
    (for _array_element_2 _allplayercontrollers
      (bind _asff_player_controller_2 (Utilities|Casting|CastToFF_PlayerController _array_element_2))
      (Default|AddPlayerInfo _asff_player_controller_2 (Variables|ServerSettings|GetConnectedPlayers)))))

(event EventPostLogin
  (params (NewPlayer :type Player%20Controller%20Object%20Reference))
  ;[1 1 1] initial setup on post login
  (Networking|SwitchHasAuthority
    (:Authority
      (bind _returnvalue (Utilities|Array|Add (Variables|ServerSettings|GetAllPlayerControllers) NewPlayer))
      (Variables|ServerSettings|SetCurrentPlayers _returnvalue)
      (bind _outactors (Actor|GetAllActorsOfClass "/Script/Engine.PlayerStart"))
      (Variables|ServerSettings|SetSpawnPoints _outactors)
      (bind _asfor_saken_gameinstance (Utilities|Casting|CastToForSakenGameinstance (Game|GetGameInstance)))
      (bind _settingvalue (Class|AdvancedSessionsLibrary|GetSessionPropertyString (.ServerSettings (Utilities|Struct|BreakServerSettings (Variables|/Game/BluePrints/All/ForSakenGameinstance.ForSakenGameinstance_C|GetServerSettings _asfor_saken_gameinstance))) "ServerName")
        (:Found
          (Variables|ServerSettings|SetServerName _settingvalue)
          (Variables|ServerSettings|SetServerMaxPlayers (Variables|/Game/BluePrints/All/ForSakenGameinstance.ForSakenGameinstance_C|GetMaxPlayers _asfor_saken_gameinstance))
          (bind _asff_player_controller (Utilities|Casting|CastToFF_PlayerController NewPlayer))
          (Default|InitialSetup _asff_player_controller))))))

(fn ConstructionScript)