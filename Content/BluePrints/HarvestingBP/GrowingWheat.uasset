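; GrowingWheat is a harvestable wheat actor that is destroyed when damage depletes its Health.
; If the damage instigator is an FF_PlayerController controlling a Base_Player, that pawn's ServerSpawnItems is called for one stackable Bundled Wheat.
; Component hits also apply fixed damage to the wheat but pass no instigator, so destruction by a hit yields no item.
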(event OnComponentHit()
  (params (HitComponent :type Primitive%20Component%20Object%20Reference) (OtherActor :type Actor%20Object%20Reference) (OtherComp :type Primitive%20Component%20Object%20Reference) (NormalImpulse :type Vector :default "0, 0, 0") (Hit :type Hit%20Result%20Structure%20%28by%20ref%29))
  (Game|Damage|ApplyDamage self 5e+01 0 0 "/Script/Engine.DamageType"))

(event EventBeginPlay)

(event Collision|EventActorBeginOverlap
  (params (OtherActor :type Actor%20Object%20Reference)))

(event EventTick
  (params (DeltaSeconds :type Float%20%28single-precision%29)))

(event Game|Damage|EventAnyDamage
  (params (Damage :type Float%20%28single-precision%29) (DamageType :type Damage%20Type%20Object%20Reference) (InstigatedBy :type Controller%20Object%20Reference) (DamageCauser :type Actor%20Object%20Reference))
  (bind _output_get (Variables|Default|SetHealth (- (Variables|Default|GetHealth) Damage)))
  (if (<= _output_get 0.0)
    (Actor|DestroyActor self)
    (bind _asff_player_controller (Utilities|Casting|CastToFF_PlayerController InstigatedBy))
    (bind _asbase_player (Utilities|Casting|CastToBase_Player (Pawn|GetControlledPawn _asff_player_controller)))
    (Default|ServerSpawnItems _asbase_player _asff_player_controller (Utilities|Struct|MakeSlotStructure (Utilities|Struct|MakeItemStructure "Bundled Wheat" "Bundled Wheat" "/Game/BluePrints/Items/thumbs/Thumb_BundledWheat.Thumb_BundledWheat" true 4 false 0.0 false 0.0 false 0.0 false false 0.0 "NewEnumerator0" false "NewEnumerator3" 0.0 false "NewEnumerator0" false "NewEnumerator0" false "NewEnumerator0" 0 false "NewEnumerator0" 0.0 "/Game/Models/Items/Nature/Wheat/WheatBunted.WheatBunted" 0 "/Game/BluePrints/Items/Nature/Item_BundledWheat.Item_BundledWheat_C" false "NewEnumerator0" 0.0) 1))))

(fn ConstructionScript)