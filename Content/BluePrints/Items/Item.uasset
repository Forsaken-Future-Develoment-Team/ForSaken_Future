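; World item actor that players can pick up, equip or consume, showing a brief on-screen prompt when a locally controlled player overlaps it.
; Interact adds it to the inventory component when the player has a backpack, otherwise to a free arm equipment slot.
; UseItem applies clamped hunger and health gains for consumables, or equips others to the right hand.
; Removal is requested through the player's ServerRemoveItem, using player index 0.
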(event Collision|EventActorBeginOverlap
  (params (OtherActor :type Actor%20Object%20Reference))
  (bind _returnvalue (Game|GetPlayerController 0))
  (bind _itemstructure (Variables|Default|GetItemStructure))
  (bind _asbase_player (Utilities|Casting|CastToBase_Player OtherActor))
  (if (Pawn|IsLocallyControlled _asbase_player)
    (if (Variables|/Game/BluePrints/Characters/Base_Player.Base_Player_C|GetHasBackPack? _asbase_player)
      (Utilities|IsValid (Variables|Default|GetscreenmessageRef)
        (:Is%20Valid
          _)
        (:Is%20Not%20Valid
          (bind _returnvalue_2 (UserInterface|CreateWidget "/Game/Ui/Ingame/messages/ScreenMessage.ScreenMessage_C" _returnvalue (Utilities|Text|ToText(String) (Utilities|String|Append "You just found a : " (Utilities|String|ToString(Text) (.name _itemstructure)) " use 'E' to pick up"))))
          (Variables|Default|SetscreenmessageRef _returnvalue_2)))
      (UserInterface|Viewport|AddtoViewport (Variables|Default|GetscreenmessageRef) 0)
      (Utilities|FlowControl|Delay 1.0)
      (Utilities|IsValid (Variables|Default|GetscreenmessageRef)
        (:Is%20Valid
          (Widget|RemovefromParent (Variables|Default|GetscreenmessageRef))
          (Variables|Default|SetscreenmessageRef 0)))
      (else
        (Utilities|IsValid (Variables|Default|GetscreenmessageRef)
          (:Is%20Valid
            _)
          (:Is%20Not%20Valid
            (bind _returnvalue_3 (UserInterface|CreateWidget "/Game/Ui/Ingame/messages/ScreenMessage.ScreenMessage_C" _returnvalue (Utilities|Text|ToText(String) (Utilities|String|Append "You just found a : " (Utilities|String|ToString(Text) (.name _itemstructure)) " use 'E' to Use if possible"))))
            (Variables|Default|SetscreenmessageRef _returnvalue_3)))
        (UserInterface|Viewport|AddtoViewport (Variables|Default|GetscreenmessageRef) 0)
        (Utilities|FlowControl|Delay 1.0)
        (Utilities|IsValid (Variables|Default|GetscreenmessageRef)
          (:Is%20Valid
            (Widget|RemovefromParent (Variables|Default|GetscreenmessageRef))
            (Variables|Default|SetscreenmessageRef 0)))))))

(event EventInteract
  (params (Interactor :type Actor%20Object%20Reference))
  (bind _asbase_player (Utilities|Casting|CastToBase_Player Interactor))
  (if (Variables|/Game/BluePrints/Characters/Base_Player.Base_Player_C|GetHasBackPack? _asbase_player)
    (bind _sucsess (Default|AddtoInventory (Actor|GetComponentbyClass Interactor "/Game/BluePrints/InventorySystem/InventoryComponent.InventoryComponent_C") (Utilities|Struct|MakeSlotStructure (Variables|Default|GetItemStructure) (Variables|Default|GetQantity))))
    (if _sucsess
      (bind _asbase_player_2 (Utilities|Casting|CastToBase_Player (Game|GetPlayerCharacter 0) :!label _label))
      (Default|ServerRemoveItem _asbase_player_2 self)
      (Utilities|IsValid (Variables|Default|GetscreenmessageRef)
        (:Is%20Valid
          (Widget|RemovefromParent (Variables|Default|GetscreenmessageRef))
          (Variables|Default|SetscreenmessageRef 0))))
    (else
      (bind _asbase_player_3 (Utilities|Casting|CastToBase_Player (Game|GetPlayerCharacter 0)))
      (if (Pawn|IsLocallyControlled _asbase_player_3)
        (if (== (.Quantity (Utilities|Struct|BreakSlotStructure (Utilities|Array|Get(acopy) (Variables|/Game/BluePrints/Characters/Base_Player.Base_Player_C|GetMyEquipment _asbase_player_3) 9))) 0)
          (Default|AddtoEqupment _asbase_player_3 9 (Utilities|Struct|MakeSlotStructure (Variables|Default|GetItemStructure) 1) (.AsPlayer%20Controller (Utilities|Casting|CastToPlayerController (Pawn|GetController _asbase_player_3))))
          (Default|UpdateEquipmentSheet _asbase_player_3)
          (goto _label)
          (elif (== (.Quantity (Utilities|Struct|BreakSlotStructure (Utilities|Array|Get(acopy) (Variables|/Game/BluePrints/Characters/Base_Player.Base_Player_C|GetMyEquipment _asbase_player_3) 8))) 0)
            (Default|AddtoEqupment _asbase_player_3 8 (Utilities|Struct|MakeSlotStructure (Variables|Default|GetItemStructure) 1) (.AsPlayer%20Controller (Utilities|Casting|CastToPlayerController (Pawn|GetController _asbase_player_3))))
            (Default|UpdateEquipmentSheet _asbase_player_3)
            (goto _label)
            (else
              (Development|PrintString "Both Arms are full"))))))))

(event EventRemoveObject
  (Utilities|IsValid (Variables|Default|GetscreenmessageRef)
    (:Is%20Valid
      (Widget|RemovefromParent (Variables|Default|GetscreenmessageRef))
      (Variables|Default|SetscreenmessageRef 0))
    (:Is%20Not%20Valid
      _))
  (Actor|DestroyActor))

(fn ConstructionScript)

(fn UseItem
  (bind _returnvalue (Game|GetPlayerCharacter 0))
  (bind _itemstructure (Variables|Default|GetItemStructure))
  (bind (_name _description _thumbnail _isstackable_ _maxstacksize _isconsumeable_ _hungerregeneratepercent _ismedical_ _healthregeneratepercent) (Utilities|Struct|BreakItemStructure _itemstructure))
  (bind _asbase_player (Utilities|Casting|CastToBase_Player (Game|GetPlayerCharacter 0)))
  ;[1 1 1] is it consumeable?
  (if _isconsumeable_
    ;[1 1 1] Set Clamped Health or Hunger, whatever is in the item
    (if (or (< (Variables|/Game/BluePrints/Characters/Base_Player.Base_Player_C|GetHunger _asbase_player) 1e+02) (< (Variables|/Game/BluePrints/Characters/Base_Player.Base_Player_C|GetHealth _asbase_player) 1e+02))
      (Variables|/Game/BluePrints/Characters/Base_Player.Base_Player_C|SetHunger _asbase_player (Math|Float|Clamp(Float) (+ (Variables|/Game/BluePrints/Characters/Base_Player.Base_Player_C|GetHunger _asbase_player) _hungerregeneratepercent) 0.0 1e+02))
      (Variables|/Game/BluePrints/Characters/Base_Player.Base_Player_C|SetHealth _asbase_player (Math|Float|Clamp(Float) (+ (Variables|/Game/BluePrints/Characters/Base_Player.Base_Player_C|GetHealth _asbase_player) _healthregeneratepercent) 0.0 1e+02))
      (Utilities|IsValid (Variables|Default|GetscreenmessageRef) :!label _label
        (:Is%20Valid
          (Widget|RemovefromParent (Variables|Default|GetscreenmessageRef))
          (Class|RemoveItemInterface|RemoveObject(Message) self)
          ;[1 1 1] Tell server to remove item and set succes for job done
          (bind _asbase_player_2 (Utilities|Casting|CastToBase_Player (Game|GetPlayerCharacter 0)))
          (Default|ServerRemoveItem _asbase_player_2 self)
          (return true))))
    (else
      (bind _asbase_player_3 (Utilities|Casting|CastToBase_Player (Game|GetPlayerCharacter 0)))
      (if (== (.Quantity (Utilities|Struct|BreakSlotStructure (Utilities|Array|Get(acopy) (Variables|/Game/BluePrints/Characters/Base_Player.Base_Player_C|GetMyEquipment _asbase_player_3) 9))) 0)
        (if (Pawn|IsLocallyControlled _returnvalue)
          (bind _asbase_player_4 (Utilities|Casting|CastToBase_Player _returnvalue))
          (bind _asbase_player_5 (Utilities|Casting|CastToBase_Player (Game|GetPlayerCharacter 0)))
          (Default|AddtoEqupment _asbase_player_5 (Variables|Default|GetRightHand) (Utilities|Struct|MakeSlotStructure (Variables|Default|GetItemStructure) 1) (.AsFF%20Player%20Controller (Utilities|Casting|CastToFF_PlayerController (Pawn|GetController _asbase_player_4))))
          (Default|ToggleInventory (Variables|/Game/BluePrints/Characters/Base_Player.Base_Player_C|GetBackPackComponent _asbase_player_5))
          (Default|ToggleInventory (Variables|/Game/BluePrints/Characters/Base_Player.Base_Player_C|GetBackPackComponent _asbase_player_5))
          (goto _label))))))