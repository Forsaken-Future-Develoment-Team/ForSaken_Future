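; Crafting table component that holds item slots and toggles a crafting widget for the locally controlled player if they have a backpack.
; PrepareCraftingTable sizes the slots and refreshes item data from class defaults.
; Added items fill partial stacks or empty slots, with overflow re-added recursively.
; CheckforItem loops through recipes, matching the first three slots by position, class and exact count, then passes the crafted item to the widget.
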(event EventBeginPlay
  (CallFunction|PrepareCraftingTable))

(fn ToggleCraftingTable
  (bind _self self)
  (bind _asbase_player (Utilities|Casting|CastToBase_Player (Game|GetPlayerCharacter 0)))
  (if (Pawn|IsLocallyControlled _asbase_player)
    (if (Variables|/Game/BluePrints/Characters/Base_Player.Base_Player_C|GetHasBackPack? _asbase_player)
      (Variables|Default|GetCraftingWidget
        (:then
          (Widget|RemovefromParent (Variables|Default|GetCraftingWidget))
          (Variables|Default|SetCraftingWidget 0)
          (Utilities|IsValid (Variables|Default|Getbackpackwindow)))
        (:else
          (CallFunction|PrepareCraftingTable)
          (bind _returnvalue (UserInterface|CreateWidget "/Game/Ui/CraftingUI/CraftingTable_W.CraftingTable_W_C" 0 (Variables|Default|GetTableName _self) _self))
          (bind _output_get (Variables|Default|SetCraftingWidget _returnvalue))
          (UserInterface|Viewport|AddtoViewport _output_get 0))))))

(fn AddtoCraftingSlots
  (params (ContentToAdd :type Slot%20Structure%20Structure))
  (if (.isstackable? (.itemstructure ContentToAdd))
    (bind _stackindex (Utilities|HasPartialStack ContentToAdd)
      (:True
        (bind _sucsess (CallFunction|AddtoStack ContentToAdd _stackindex))
        (if _sucsess
          _
          (else
            (Development|PrintString "doesnt work on partial")
            (return false))))
      (:False
        (bind _sucsess_2 (CallFunction|CreateStack ContentToAdd :!label _label))
        (if _sucsess_2
          _
          (else
            (Development|PrintString "cant seem to add")
            (return false)))))
    (else
      (goto _label)))
  (return true))

(fn PrepareCraftingTable
  (bind _craftingslots (Variables|Default|GetCraftingSlots))
  (Utilities|Array|Resize (Variables|Default|GetCraftingSlots) (Variables|Default|GetNumberOfCraftingSlots))
  (for (_array_element _array_index) (Variables|Default|GetCraftingSlots)
    (if (< (.quantity _array_element) 1)
      (bind _structout (Utilities|Struct|SetmembersinSlotStructure (Utilities|Array|Get(acopy) (Variables|Default|GetCraftingSlots) _array_index) (Utilities|Struct|MakeItemStructure "" "" 0 false 0 false 0.0 false 0.0 false 0.0 false false 0.0 "NewEnumerator0" false "NewEnumerator3" 0.0 false "NewEnumerator0" false "NewEnumerator0" false "NewEnumerator0" 0 false "NewEnumerator0" 0.0 0 0 0 false "NewEnumerator0" 0.0)))
      (Utilities|Array|SetArrayElem _craftingslots _array_index _structout)
      (elif (!= (.Class (Utilities|Struct|BreakItemStructure (.itemstructure _array_element))) 0)
        (Utilities|Array|SetArrayElem _craftingslots _array_index (Utilities|Struct|MakeSlotStructure (.ItemStructure (Utilities|GetClassDefaults (.Class (Utilities|Struct|BreakItemStructure (.itemstructure _array_element))))) (.quantity _array_element)))))))

(fn CreateStack
  (params (ContentToAdd :type Slot%20Structure%20Structure))
  (bind (_array_element _array_index) (Utilities|Array|ForEachLoopwithBreak (Variables|Default|GetCraftingSlots) :!label _label)
    (:LoopBody
      (if (<= (.quantity _array_element) 0)
        (LocalVariables|SetHasSpace? true)
        (goto _label Break)))
    (:Completed
      (if (LocalVariables|GetHasSpace?)
        (Utilities|Array|SetArrayElem (Variables|Default|GetCraftingSlots) _array_index ContentToAdd)
        (return (LocalVariables|GetHasSpace?))
        (else
          (return false))))))

(fn AddtoStack
  (params (SlotStructure :type Slot%20Structure%20Structure) (SlotIndex :type Integer))
  (bind _craftingslots (Variables|Default|GetCraftingSlots))
  (bind _craftingslots_2 (Variables|Default|GetCraftingSlots))
  (bind _maxstacksize (Utilities|Struct|BreakItemStructure (.itemstructure SlotStructure)))
  (bind _output (Utilities|Array|Get(acopy) _craftingslots SlotIndex))
  (bind _output_2 (Utilities|Array|Get(acopy) _craftingslots_2 SlotIndex))
  (bind _output_get (LocalVariables|SetCurrentQuantity (.quantity _output)))
  (if (> (+ _output_get (.Quantity (Utilities|Struct|BreakSlotStructure SlotStructure))) (.maxstacksize (.itemstructure _output)))
    (Utilities|Array|SetArrayElem (Variables|Default|GetCraftingSlots) SlotIndex (Utilities|Struct|MakeSlotStructure (.itemstructure SlotStructure) _maxstacksize))
    (CallFunction|AddtoCraftingSlots (Utilities|Struct|MakeSlotStructure (.itemstructure SlotStructure) (- (.quantity SlotStructure) (- _maxstacksize (LocalVariables|GetCurrentQuantity)))))
    (else
      (Utilities|Array|SetArrayElem _craftingslots_2 SlotIndex (Utilities|Struct|MakeSlotStructure (.itemstructure _output_2) (+ (.quantity SlotStructure) (.quantity _output_2))))))
  (return true))

(fn CraftingQuery
  (params (ItemClass :type Item%20Class%20Reference) (QueryAmount :type Integer))
  ;[1 1 1] ok so this function we can check if the item we're looking for is in the craftingslots
  (bind _array_element (Utilities|Array|ForEachLoopwithBreak (Variables|Default|GetCraftingSlots))
    (:LoopBody
      (if (== (.Class (Utilities|Struct|BreakItemStructure (.itemstructure _array_element))) ItemClass)
        (LocalVariables|SetRunningTotal (+ (.quantity _array_element) (LocalVariables|GetRunningTotal)))))
    (:Completed
      (if (>= QueryAmount (LocalVariables|GetRunningTotal))
        (return true)
        (else
          (return false))))))

(fn CheckforItem
  (bind _craftingslots (Variables|Default|GetCraftingSlots))
  (bind _craftingwidget (Variables|Default|GetCraftingWidget))
  (bind _craftingwidget_2 (Variables|Default|GetCraftingWidget))
  (bind _output (Utilities|Array|Get(acopy) _craftingslots 2))
  (bind _output_2 (Utilities|Array|Get(acopy) _craftingslots))
  (bind _output_3 (Utilities|Array|Get(acopy) _craftingslots 1))
  (bind (_itemstructure _quantity) (Utilities|Struct|BreakSlotStructure _output))
  (bind (_itemstructure_2 _quantity_2) (Utilities|Struct|BreakSlotStructure _output_2))
  (bind (_itemstructure_3 _quantity_3) (Utilities|Struct|BreakSlotStructure _output_3))
  (if (and (== (.Class (Utilities|Struct|BreakItemStructure _itemstructure_2)) (.Item1 (Utilities|Struct|BreakRecieptsStruct (Utilities|Array|Get(acopy) (Variables|Default|GetRecieptArray) (Variables|Default|GetRecieptIndex))))) (== (.ITem1Count (Utilities|Struct|BreakRecieptsStruct (Utilities|Array|Get(acopy) (Variables|Default|GetRecieptArray) (Variables|Default|GetRecieptIndex)))) _quantity_2)) :!label _label
    (Variables|Default|SetItem1 true)
    (else
      (Variables|Default|SetItem1 false)))
  (if (and (== (.Item2Count (Utilities|Struct|BreakRecieptsStruct (Utilities|Array|Get(acopy) (Variables|Default|GetRecieptArray) (Variables|Default|GetRecieptIndex)))) _quantity_3) (== (.Class (Utilities|Struct|BreakItemStructure _itemstructure_3)) (.Item2 (Utilities|Struct|BreakRecieptsStruct (Utilities|Array|Get(acopy) (Variables|Default|GetRecieptArray) (Variables|Default|GetRecieptIndex))))))
    (Variables|Default|SetItem2 true)
    (else
      (Variables|Default|SetItem2 false)))
  (if (and (== (.Class (Utilities|Struct|BreakItemStructure _itemstructure)) (.Item3 (Utilities|Struct|BreakRecieptsStruct (Utilities|Array|Get(acopy) (Variables|Default|GetRecieptArray) (Variables|Default|GetRecieptIndex))))) (== (.Item3Count (Utilities|Struct|BreakRecieptsStruct (Utilities|Array|Get(acopy) (Variables|Default|GetRecieptArray) (Variables|Default|GetRecieptIndex)))) _quantity))
    (Variables|Default|SetItem3 true)
    (else
      (Variables|Default|SetItem3 false)))
  (if (Math|Boolean|ANDBoolean (Variables|Default|GetItem1) (Variables|Default|GetItem2) (Variables|Default|GetItem3))
    (bind _output_get (Variables|Default|SetGivenItem (.CraftedItem (Utilities|Struct|BreakRecieptsStruct (Utilities|Array|Get(acopy) (Variables|Default|GetRecieptArray) (Variables|Default|GetRecieptIndex))))))
    (Variables|/Game/Ui/CraftingUI/CraftingTable_W.CraftingTable_W_C|SetGivenItem _craftingwidget _output_get)
    (Variables|/Game/Ui/CraftingUI/CraftingTable_W.CraftingTable_W_C|SetIsItem _craftingwidget true)
    (Variables|Default|SetItem1 false)
    (Variables|Default|SetItem2 false)
    (Variables|Default|SetItem3 false)
    (Variables|Default|SetRecieptIndex 0)
    (elif (== (Variables|Default|GetRecieptIndex) (Variables|Default|GetMaxReciept))
      (Variables|/Game/Ui/CraftingUI/CraftingTable_W.CraftingTable_W_C|SetGivenItem _craftingwidget_2 "")
      (Variables|/Game/Ui/CraftingUI/CraftingTable_W.CraftingTable_W_C|SetIsItem _craftingwidget_2 false)
      (Variables|Default|SetItem1 false)
      (Variables|Default|SetItem2 false)
      (Variables|Default|SetItem3 false)
      (Variables|Default|SetRecieptIndex 0)
      (else
        (Variables|Default|SetRecieptIndex (Math|Integer|Clamp(Integer) (+ (Variables|Default|GetRecieptIndex) 1) 0 (Variables|Default|GetMaxReciept)))
        (goto _label)))))