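; Flour grinder crafting station that players with a backpack can use to produce a sack of flour.
; Overlap shows a brief prompt, and Interact toggles the inventory alongside a grinder widget whose input slot loads from SlotContent.
; Walking away saves that slot and closes the widget.
; GrindFlour plays the animation, adds flour to the backpack, clears the slot and double-toggles the inventory, apparently to refresh it.
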(event Custom|GrindFlour
  (bind _widgetref (Variables|Default|GetWidgetRef))
  (bind _flourgrinderinslot (Variables|/Game/Ui/FlourGrinderUi/FlourGrinderWidget.FlourGrinderWidget_C|GetFlourGrinderInSlot _widgetref))
  (Components|Animation|PlayAnimation (Variables|Default|GetSkeletalMesh) "/Game/Models/MapObjects/Machines/FlourGrinder/FlourGrinder_Anim.FlourGrinder_Anim" false)
  (bind _asbase_player (Utilities|Casting|CastToBase_Player (Game|GetPlayerCharacter 0)))
  (Default|AddtoInventory (Variables|/Game/BluePrints/Characters/Base/Base_Player.Base_Player_C|GetBackPackComponent _asbase_player) (Utilities|Struct|MakeSlotStructure (Utilities|Struct|MakeItemStructure "sack of flour" "sack of flour" "/Game/BluePrints/Items/thumbs/Thumb_flourBag.Thumb_flourBag" false 1 false 0.0 false 0.0 false 0.0 false false 0.0 "NewEnumerator0" false "NewEnumerator3" 0.0 false "NewEnumerator0" false "NewEnumerator0" false "NewEnumerator0" 0 false "NewEnumerator0" 0.0 "/Game/Models/Items/Food/Flour/Flourbag.Flourbag" 0 "/Game/BluePrints/Items/Food/Item_FlourBag.Item_FlourBag_C") 1))
  (Variables|/Game/Ui/FlourGrinderUi/FlourGrinderInSlot.FlourGrinderInSlot_C|SetSlotStructure _flourgrinderinslot "")
  (Default|UpdateSlot _flourgrinderinslot)
  (bind _asbase_player_2 (Utilities|Casting|CastToBase_Player (Game|GetPlayerCharacter 0)))
  (Default|ToggleInventory (Variables|/Game/BluePrints/Characters/Base/Base_Player.Base_Player_C|GetBackPackComponent _asbase_player_2))
  (Default|ToggleInventory (Variables|/Game/BluePrints/Characters/Base/Base_Player.Base_Player_C|GetBackPackComponent _asbase_player_2)))

(event Collision|EventActorBeginOverlap
  (params (OtherActor :type Actor%20Object%20Reference))
  (bind _asbase_player (Utilities|Casting|CastToBase_Player OtherActor))
  (if (Variables|/Game/BluePrints/Characters/Base/Base_Player.Base_Player_C|GetHasBackPack? _asbase_player)
    (bind _returnvalue (UserInterface|CreateWidget "/Game/Ui/Ingame/messages/ScreenMessage.ScreenMessage_C" (Variables|/Game/BluePrints/Characters/Base/Base_Player.Base_Player_C|GetControllerRef _asbase_player) "You found a FlourGrinder, press 'E' to Interact with it"))
    (bind _output_get (Variables|Default|SetScreenmessageref _returnvalue))
    (UserInterface|Viewport|AddtoViewport _output_get 0)
    (Utilities|FlowControl|Delay 1.0)
    (Utilities|IsValid (Variables|Default|GetScreenmessageref)
      (:Is%20Valid
        (Widget|RemovefromParent (Variables|Default|GetScreenmessageref))
        (Variables|Default|SetScreenmessageref 0)))
    (else
      (bind _returnvalue_2 (UserInterface|CreateWidget "/Game/Ui/Ingame/messages/ScreenMessage.ScreenMessage_C" (Variables|/Game/BluePrints/Characters/Base/Base_Player.Base_Player_C|GetControllerRef _asbase_player) "You need a BackPack to interact with the Grinder"))
      (bind _output_get_2 (Variables|Default|SetScreenmessageref _returnvalue_2))
      (UserInterface|Viewport|AddtoViewport _output_get_2 0)
      (Utilities|FlowControl|Delay 1.0)
      (Utilities|IsValid (Variables|Default|GetScreenmessageref)
        (:Is%20Valid
          (Widget|RemovefromParent (Variables|Default|GetScreenmessageref))
          (Variables|Default|SetScreenmessageref 0))))))

(event EventTick
  (params (DeltaSeconds :type Float%20%28single-precision%29)))

(event Collision|EventActorEndOverlap
  (params (OtherActor :type Actor%20Object%20Reference))
  (Utilities|Casting|CastToBase_Player OtherActor)
  (Utilities|IsValid (Variables|Default|GetWidgetRef)
    (:Is%20Valid
      (Utilities|Array|SetArrayElem (Variables|Default|GetSlotContent) 0 (Variables|/Game/Ui/FlourGrinderUi/FlourGrinderInSlot.FlourGrinderInSlot_C|GetSlotStructure (Variables|/Game/Ui/FlourGrinderUi/FlourGrinderWidget.FlourGrinderWidget_C|GetFlourGrinderInSlot (Variables|Default|GetWidgetRef))))
      (Widget|RemovefromParent (Variables|Default|GetWidgetRef))
      (Variables|Default|SetWidgetRef 0)
      (Utilities|IsValid (Variables|Default|GetScreenmessageref)
        (:Is%20Valid
          (Widget|RemovefromParent (Variables|Default|GetScreenmessageref))
          (Variables|Default|SetScreenmessageref 0))))))

(event EventInteract
  (params (Interactor :type Actor%20Object%20Reference))
  (bind _slotcontent (Variables|Default|GetSlotContent))
  (bind _asbase_player (Utilities|Casting|CastToBase_Player Interactor))
  (if (Variables|/Game/BluePrints/Characters/Base/Base_Player.Base_Player_C|GetHasBackPack? _asbase_player)
    (Utilities|IsValid (Variables|Default|GetWidgetRef)
      (:Is%20Valid
        (bind _asbase_player_2 (Utilities|Casting|CastToBase_Player Interactor))
        (Default|ToggleInventory (Variables|/Game/BluePrints/Characters/Base/Base_Player.Base_Player_C|GetBackPackComponent _asbase_player_2))
        (Widget|RemovefromParent (Variables|Default|GetWidgetRef))
        (Variables|Default|SetWidgetRef 0))
      (:Is%20Not%20Valid
        (bind _asbase_player_3 (Utilities|Casting|CastToBase_Player Interactor))
        (Default|ToggleInventory (Variables|/Game/BluePrints/Characters/Base/Base_Player.Base_Player_C|GetBackPackComponent _asbase_player_3))
        (bind _returnvalue (UserInterface|CreateWidget "/Game/Ui/FlourGrinderUi/FlourGrinderWidget.FlourGrinderWidget_C" (Variables|/Game/BluePrints/Characters/Base/Base_Player.Base_Player_C|GetControllerRef _asbase_player_3)))
        (bind _output_get (Variables|Default|SetWidgetRef _returnvalue))
        (bind _output_get_2 (Variables|/Game/Ui/FlourGrinderUi/FlourGrinderInSlot.FlourGrinderInSlot_C|SetSlotStructure (Variables|/Game/Ui/FlourGrinderUi/FlourGrinderWidget.FlourGrinderWidget_C|GetFlourGrinderInSlot _output_get) (Utilities|Array|Get(acopy) _slotcontent)))
        (Utilities|Array|SetArrayElem _slotcontent 0 _output_get_2)
        (UserInterface|Viewport|AddtoViewport _returnvalue 0)))))

(fn ConstructionScript)