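; Crafting table actor that players interact with to open or close crafting alongside their backpack inventory.
; On overlap, a locally controlled player with a backpack sees a short on-screen prompt, removed after a delay or when overlap ends.
; Interact flips the local player's IsCrafting flag, then toggles the CraftingTableComponent and the inventory on the first player character's BackPackComponent.
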(event EventBeginPlay)

(event Collision|EventActorBeginOverlap
  (params (OtherActor :type Actor%20Object%20Reference))
  (bind _asbase_player (Utilities|Casting|CastToBase_Player OtherActor))
  (if (Pawn|IsLocallyControlled _asbase_player)
    (if (Variables|/Game/BluePrints/Characters/Base/Base_Player.Base_Player_C|GetHasBackPack? _asbase_player)
      (bind _returnvalue (UserInterface|CreateWidget "/Game/Ui/Ingame/messages/ScreenMessage.ScreenMessage_C" 0 "You found a crafting table, press 'E' to interact"))
      (Variables|Default|SetScreenMessageRef _returnvalue)
      (UserInterface|Viewport|AddtoViewport (Variables|Default|GetScreenMessageRef) 0)
      (Utilities|FlowControl|Delay 1.0)
      (Utilities|IsValid (Variables|Default|GetScreenMessageRef)
        (:Is%20Valid
          (Widget|RemovefromParent (Variables|Default|GetScreenMessageRef))
          (Variables|Default|SetScreenMessageRef 0))))))

(event Collision|EventActorEndOverlap
  (params (OtherActor :type Actor%20Object%20Reference))
  (bind _screenmessageref (Variables|Default|GetScreenMessageRef))
  (bind _asbase_player (Utilities|Casting|CastToBase_Player OtherActor))
  (if (Pawn|IsLocallyControlled _asbase_player)
    (Utilities|IsValid _screenmessageref
      (:Is%20Valid
        (Widget|RemovefromParent _screenmessageref)))))

(event EventInteract
  (params (Interactor :type Actor%20Object%20Reference))
  (bind _asbase_player (Utilities|Casting|CastToBase_Player Interactor))
  (if (Pawn|IsLocallyControlled _asbase_player)
    (if (Variables|/Game/BluePrints/Characters/Base/Base_Player.Base_Player_C|GetIsCrafting? _asbase_player)
      (Variables|/Game/BluePrints/Characters/Base/Base_Player.Base_Player_C|SetIsCrafting? _asbase_player false)
      (else
        (Variables|/Game/BluePrints/Characters/Base/Base_Player.Base_Player_C|SetIsCrafting? _asbase_player true)))
    (Default|ToggleCraftingTable (Variables|Default|GetCraftingTableComponent))
    (bind _asbase_player_2 (Utilities|Casting|CastToBase_Player (Game|GetPlayerCharacter 0)))
    (Default|ToggleInventory (Variables|/Game/BluePrints/Characters/Base/Base_Player.Base_Player_C|GetBackPackComponent _asbase_player_2))))

(fn ConstructionScript)