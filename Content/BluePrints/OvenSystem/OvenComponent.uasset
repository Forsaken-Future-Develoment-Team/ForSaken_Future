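; Oven component that lets the local player with a backpack cook food through an oven widget.
; ToggleOven opens or closes the widget alongside the backpack inventory and sets the player's IsCooking flag.
; CanCook enables cooking when slot 0 matches a recipe input and slot 1 holds stick or coal fuel.
; StartCooking instantly adds the recipe output to the backpack, then, if successful, clears both slots and refreshes the UI.
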(event EventBeginPlay)

(fn ToggleOven
  (bind _self self)
  (bind _asbase_player (Utilities|Casting|CastToBase_Player (Game|GetPlayerCharacter 0)))
  (if (Pawn|IsLocallyControlled _asbase_player)
    (bind _asbase_player_2 (Utilities|Casting|CastToBase_Player (Game|GetPlayerCharacter 0)))
    (if (Variables|/Game/BluePrints/Characters/Base_Player.Base_Player_C|GetHasBackPack? _asbase_player_2)
      (Variables|Default|GetOvenWindow
        (:then
          (Widget|RemovefromParent (Variables|Default|GetOvenWindow))
          (Variables|Default|SetOvenWindow 0)
          (bind _asbase_player_3 (Utilities|Casting|CastToBase_Player (Game|GetPlayerCharacter 0)))
          (Default|ToggleInventory (Variables|/Game/BluePrints/Characters/Base_Player.Base_Player_C|GetBackPackComponent _asbase_player_3))
          (Variables|/Game/BluePrints/Characters/Base_Player.Base_Player_C|SetIsCooking? _asbase_player_3 false))
        (:else
          (bind _asplayer_controller (Utilities|Casting|CastToPlayerController (Pawn|GetController _asbase_player_2)))
          (bind _returnvalue (UserInterface|CreateWidget "/Game/Ui/OvenUi/OvenWidget.OvenWidget_C" _asplayer_controller (Variables|Default|GetOvenName _self) _self))
          (bind _output_get (Variables|Default|SetOvenWindow _returnvalue))
          (UserInterface|Viewport|AddtoViewport _output_get 0)
          (bind _asbase_player_4 (Utilities|Casting|CastToBase_Player (Game|GetPlayerCharacter 0)))
          (Default|ToggleInventory (Variables|/Game/BluePrints/Characters/Base_Player.Base_Player_C|GetBackPackComponent _asbase_player_4))
          (Variables|/Game/BluePrints/Characters/Base_Player.Base_Player_C|SetIsCooking? _asbase_player_4 true))))))

(fn CanCook?
  (bind _ovenslots (Variables|Default|GetOvenSlots))
  (bind _output (Utilities|Array|Get(acopy) _ovenslots 1))
  (bind _itemstructure (Utilities|Struct|BreakSlotStructure _output))
  (for _array_element (Variables|Default|GetCookingReciepts)
    (if (and (== (.FoodIn (Utilities|Struct|BreakFoodReciept _array_element)) (.class (.ItemStructure (Utilities|Struct|BreakSlotStructure (Utilities|Array|Get(acopy) _ovenslots))))) (Math|Boolean|ORBoolean (== (.class _itemstructure) "/Game/BluePrints/Items/Nature/Item_Stick.Item_Stick_C") (== (.class _itemstructure) "/Game/BluePrints/Items/Miningstuff/Item_Coal.Item_Coal_C") (== (.class _itemstructure) "/Game/BluePrints/Items/Miningstuff/Item_Coal.Item_Coal_C")))
      (Variables|/Game/Ui/OvenUi/OvenWidget.OvenWidget_C|SetCanCook? (Variables|Default|GetOvenWindow) true))))

(fn StartCooking
  (bind _ovenslots (Variables|Default|GetOvenSlots))
  (bind _array_element (Utilities|Array|ForEachLoopwithBreak (Variables|Default|GetCookingReciepts) :!label _label)
    (:LoopBody
      (if (== (.class (.ItemStructure (Utilities|Struct|BreakSlotStructure (Utilities|Array|Get(acopy) (Variables|Default|GetOvenSlots))))) (.FoodIn (Utilities|Struct|BreakFoodReciept _array_element)))
        (goto _label Break)))
    (:Completed
      (bind _asbase_player (Utilities|Casting|CastToBase_Player (Game|GetPlayerCharacter 0)))
      (bind _sucsess (Default|AddtoInventory (Variables|/Game/BluePrints/Characters/Base_Player.Base_Player_C|GetBackPackComponent _asbase_player) (Utilities|Struct|MakeSlotStructure (.ItemStructure (Utilities|Struct|BreakSlotStructure (.FoodOut (Utilities|Struct|BreakFoodReciept _array_element)))) (.Quantity (Utilities|Struct|BreakSlotStructure (.FoodOut (Utilities|Struct|BreakFoodReciept _array_element)))))))
      (if _sucsess
        (Variables|/Game/Ui/OvenUi/OvenWidget.OvenWidget_C|SetCanCook? (Variables|Default|GetOvenWindow) false)
        (Utilities|Array|SetArrayElem :TargetArray _ovenslots)
        (Utilities|Array|SetArrayElem :TargetArray _ovenslots :Index 1)
        (Default|RefreshAfterCooking (Variables|Default|GetOvenWindow))
        (bind _asbase_player_2 (Utilities|Casting|CastToBase_Player (Game|GetPlayerCharacter 0)))
        (Default|ToggleInventory (Variables|/Game/BluePrints/Characters/Base_Player.Base_Player_C|GetBackPackComponent _asbase_player_2))
        (Default|ToggleInventory (Variables|/Game/BluePrints/Characters/Base_Player.Base_Player_C|GetBackPackComponent _asbase_player_2))))))